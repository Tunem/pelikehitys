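; Rock obstacle actor that reacts to overlapping Hugo or a respawn trigger.
; On overlap it checks the other actor's object name, calling the RockHitED dispatcher for a Hugo hit and otherwise running the respawn check.
; After any overlap it teleports back to RockLoc via ResetPosition.
; ApplyEffect and ResetScaleAndValue are empty here, and BeginPlay and Tick are disabled.
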(event `self.ReceiveActorBeginOverlap`
  (params (OtherActor :type "Actor Object Reference"))
  (bind _returnvalue (`KismetSystemLibrary.GetObjectName` OtherActor))
  ;[1 1 1] Check Hit
  (bind _hit_result (`self.CheckHugoHit` _returnvalue))
  (if _hit_result
    ;[1 1 1] Broadcast message
    (`self.RockHit_ED`)
    (else
      ;[1 1 1] If not Hugo, check respawntrigger
      (`self.CheckRespawnHit` _returnvalue)))
  ;[1 1 1] Reset
  (`self.ResetPosition`)
  (`self.ResetScaleAndValue`))

(fn `Apply Effect`)

(fn `ResetPosition`
  (`self.K2_SetActorLocation` (`self.rockLoc`)))

(fn `ResetScaleAndValue`)

(fn `UserConstructionScript`
  (`parent.UserConstructionScript`))