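; MoneyCoin is a collectible coin pickup that awards money when Hugo touches it.
; On overlap it checks the other actor's name for Hugo, then plays a hit sound and broadcasts its Value through the money-collected dispatcher.
; Other overlaps go through a respawn-trigger check, and every overlap ends by resetting position, scale and value, so the coin is reused.
; Tick and ApplyEffect only call the parent.
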(event `self.ReceiveActorBeginOverlap`
  (params (OtherActor :type "Actor Object Reference"))
  (bind _returnvalue (`KismetSystemLibrary.GetObjectName` OtherActor))
  ;[1 1 1] Check Hit
  (bind _hit_result (`self.CheckHugoHit` _returnvalue))
  (if _hit_result
    ;[1 1 1] Broadcast message
    (`GameplayStatics.PlaySound2D` "/Game/Sounds/Coin_hit.Coin_hit" 1.0 1.0 0.0 null null)
    (`self.MoneyCollected_ED` (`self.Value`))
    (else
      ;[1 1 1] If not Hugo, check respawntrigger
      (`self.CheckRespawnHit` _returnvalue)))
  ;[1 1 1] Reset
  (`self.ResetPosition`)
  (`self.ResetScaleAndValue`))

(event `self.ReceiveTick`
  (params (DeltaSeconds :type "Float (single-precision)"))
  (`parent.ReceiveTick` 0.0))

(fn `Apply Effect`
  (`parent.Apply Effect`))

(fn `UserConstructionScript`)